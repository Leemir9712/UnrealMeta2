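; BP_mypawn is a HelloUnreal pawn that acts as an on-screen elapsed-time counter, showing minutes and seconds with Korean unit labels.
; Tick feeds delta time to PrintTime, which accumulates it and prints only when the formatted string changes.
; FloToStr00 floors and zero-pads each field, while the similar IntToStr00 helper is unused.
; BeginPlay's display-name print has both screen and log output disabled.
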(event EventBeginPlay
  (Development|PrintString (Utilities|GetDisplayName self) false false "(R=0.000000,G=0.660000,B=1.000000,A=1.000000)" 6e+01))

(event EventTick
  (params (DeltaSeconds :type Float%20%28single-precision%29))
  ;[1 1 1] 00MIN 00SEC
  (CallFunction|PrintTime (* DeltaSeconds 1.0)))

(fn ConstructionScript)

(fn InttoStr00
  (params (Number :type Integer))
  (bind _returnvalue (Utilities|String|ToString(Integer) Number))
  (if (< Number 10)
    (return (Utilities|String|Append "0" _returnvalue))
    (else
      (return _returnvalue))))

(fn FlotoStr00
  (params (Number :type Float%20%28single-precision%29))
  (bind _returnvalue (Math|Float|Floor Number))
  (bind _returnvalue_2 (Utilities|String|ToString(Integer) _returnvalue))
  (if (< _returnvalue 10)
    (return (Utilities|String|Append "0" _returnvalue_2) 0.0)
    (else
      (return _returnvalue_2 0.0))))

(fn PrintTime
  (params (DeltaSeconds :type Float%20%28single-precision%29))
  (bind _output_get (Variables|Default|SetTotalDeltaSec (+ (Variables|Default|GetTotalDeltaSec) DeltaSeconds)))
  (if (Utilities|Enum|NotEqual(Enum) (Utilities|String|Append (.String (Leemir|FlotoStr00 (/ _output_get 6e+01))) "분" (.String (Leemir|FlotoStr00 (Math|Float|%(Float) _output_get 6e+01))) "초") (Variables|Default|GetBeforeString))
    (Development|PrintString (Utilities|String|Append (.String (Leemir|FlotoStr00 (/ _output_get 6e+01))) "분" (.String (Leemir|FlotoStr00 (Math|Float|%(Float) _output_get 6e+01))) "초"))
    (Variables|Default|SetBeforeString (Utilities|String|Append (.String (Leemir|FlotoStr00 (/ _output_get 6e+01))) "분" (.String (Leemir|FlotoStr00 (Math|Float|%(Float) _output_get 6e+01))) "초"))))