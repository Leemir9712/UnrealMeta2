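; BP_Potal is a portal actor whose sphere appears once every coin in its Coin array is hidden.
; The Sphere starts invisible on BeginPlay.
; EventGetCoin prints a debug string, then sets the sphere's visibility from CheckAllCoinHide, which loops over the coins and returns false at the first one not flagged IsCoinHide.
; Only visibility changes here; the file holds no overlap or teleport logic.
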(event EventBeginPlay
  (Rendering|SetVisibility (Variables|Default|GetSphere) false false))

(fn ConstructionScript)

(fn EventGetCoin
  (Development|PrintString "EventGetCoin")
  (bind _isallhide (CallFunction|CheckAllCoinHide))
  (Rendering|SetVisibility (Variables|Default|GetSphere) _isallhide false))

(fn CheckAllCoinHide
  (for _array_element (Variables|Default|GetCoin)
    (if (not (Variables|/Game/Collision/Blueprints/BP_Coin.BP_Coin_C|GetIsCoinHide _array_element))
      (return false)))
  (return true))